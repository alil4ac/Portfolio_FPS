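; BP_PlayerController is the player controller that turns Enhanced Input actions into movement and look for the controlled pawn.
; BeginPlay adds the IMC_PlayerInput mapping context, and IA_Move drives movement input rotated by control yaw only.
; IA_LookX feeds controller yaw, while IA_LookY hands pitch to BP_Playerable's SetCameraPitch, leaving an AddPitchInput node unused.
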(event `self.ReceiveBeginPlay`
  (`EnhancedInputSubsystemInterface.AddMappingContext` (subsystem `EnhancedInputLocalPlayerSubsystem`) "/Game/InputAction/IMC_PlayerInput.IMC_PlayerInput" 0 (struct)))

(event `EnhancedInput|/Game/InputAction/IA_Move`
  (params (ActionValue :type "Vector Structure") (ElapsedSeconds :type "Float (double-precision)") (TriggeredSeconds :type "Float (double-precision)") (InputAction :type "InputAction Object Reference" :default "/Game/InputAction/IA_Move.IA_Move"))
  (bind (_returnvalue_roll _returnvalue_pitch _returnvalue_yaw) (`KismetMathLibrary.BreakRotator` (`self.GetControlRotation`)))
  (:`Triggered`
    (`Pawn.AddMovementInput` (`self.K2_GetPawn`) (`KismetMathLibrary.GreaterGreater_VectorRotator` ActionValue (`KismetMathLibrary.MakeRotator` 0.0 0.0 _returnvalue_yaw)) 1.0 false)))

(event `EnhancedInput|/Game/InputAction/IA_LookX`
  (params (ActionValue :type "Vector Structure") (ElapsedSeconds :type "Float (double-precision)") (TriggeredSeconds :type "Float (double-precision)") (InputAction :type "InputAction Object Reference" :default "/Game/InputAction/IA_LookX.IA_LookX"))
  (:`Triggered`
    (`self.AddYawInput` ActionValue_Z)))

(event `EnhancedInput|/Game/InputAction/IA_LookY`
  (params (ActionValue :type "Vector Structure") (ElapsedSeconds :type "Float (double-precision)") (TriggeredSeconds :type "Float (double-precision)") (InputAction :type "InputAction Object Reference" :default "/Game/InputAction/IA_LookY.IA_LookY"))
  (:`Triggered`
    (`/Game/BluePrint/Characters/BP_Playerable.SetCameraPitch` (cast `/Game/BluePrint/Characters/BP_Playerable` (`self.K2_GetPawn`) :!pure true) ActionValue_Y)))

(fn `UserConstructionScript`)