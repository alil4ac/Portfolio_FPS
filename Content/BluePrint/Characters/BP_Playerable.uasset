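; BP_Playerable is a playable character Blueprint that equips a weapon and controls the pitch of its spring-arm camera.
; BeginPlay spawns the WeaponType actor, attaches it to the mesh's hand_r_weapon socket, then calls SetTransformMessage on it.
; SetCameraPitch adds the input to the current arm pitch through a clamped math expression and applies it to the spring arm, while GetCameraPitch reads that pitch back.
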(event EventBeginPlay
  (|CallParentFunction)
  (bind _returnvalue (Game|SpawnActorfromClass (Variables|Default|GetWeaponType) (Math|Transform|MakeTransform "0, 0, 0") "Undefined" "MultiplyWithRoot" self 0))
  (Transformation|AttachComponentToComponent _returnvalue (Variables|Character|GetMesh) "hand_r_weapon" "SnapToTarget" "KeepRelative" "SnapToTarget" true)
  (Class|BPIWeapon|SetTransform(Message) _returnvalue))

(fn ConstructionScript
  (|CallParentFunction))

(fn SetCameraPitch
  (params (Pitch :type Float%20%28double-precision%29))
  (LocalVariables|SetArmPitch (.pitch (Class|SpringArmComponent|GetTargetRotation (Variables|Default|GetSpringArm))))
  (Transformation|SetRelativeRotation (Variables|Default|GetSpringArm) (Math|Rotator|MakeRotator 0.0 (|(Clamp(({7710B8FA-48BD-4865-8FC0-8F9008B75571}+Pitch),{774B7F66-41DD-2D1D-E3A2-A4A6CD64C5C5},{4E352361-4946-2478-C37B-72AB4D254BBB})) Pitch) 0.0) false false)
  (return))

(fn GetCameraPitch
  (bind _springarm (Variables|Default|GetSpringArm)
    (:then
      (return (.pitch (Class|SpringArmComponent|GetTargetRotation _springarm))))
    (:else)))